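; BP_Projectile is a projectile actor that flies toward a target location and damages enemies it hits.
; On BeginPlay it sets movement velocity straight at the target and scales the damage component's damage by a multiplier.
; Overlapping an enemy passes it to the damage component and destroys the projectile.
; Tick also destroys it once it comes close to the target point, so it does not track moving targets.
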(event `self.ReceiveBeginPlay`
  (bind _bp_damagecomponent (`self.BP_DamageComponent`))
  (set `MovementComponent.Velocity` (* (`KismetMathLibrary.Normal` (- (`self.TargetLocation`) (`self.K2_GetActorLocation`))) (`self.ProjectileSpeed`)) (`self.ProjectileMovement`))
  (set `/Game/CustomAguilar/Components/BP_DamageComponent.Damage` (* (`/Game/CustomAguilar/Components/BP_DamageComponent.Damage` _bp_damagecomponent) (`self.DamageMultiplier`)) _bp_damagecomponent))

(event `self.ReceiveTick`
  (params (DeltaSeconds :type "Float (single-precision)"))
  (if (<= (`KismetMathLibrary.Vector_Distance` (`self.K2_GetActorLocation`) (`self.TargetLocation`)) 30.0)
    (`self.K2_DestroyActor`)))

(event `self.SphereCollision.OnComponentBeginOverlap`
  (params (OverlappedComponent :type "PrimitiveComponent Object Reference") (OtherActor :type "Actor Object Reference") (OtherComp :type "PrimitiveComponent Object Reference") (OtherBodyIndex :type Integer) (bFromSweep :type Boolean) (SweepResult :type "HitResult Structure (by ref)"))
  (bind _asbp_enemy_base (cast `/Game/CustomAguilar/Enemies/BP_EnemyBase` OtherActor))
  (`/Game/CustomAguilar/Components/BP_DamageComponent.GetDamage` (`self.BP_DamageComponent`) _asbp_enemy_base)
  (`self.K2_DestroyActor`))

(fn `UserConstructionScript`)