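; Upgrade inventory actor for the top-down player that stores upgrades up to a slot limit and applies their stat bonuses.
; On BeginPlay it caches the player and base walk speed, then creates the inventory HUD widget.
; AddUpgrade stores and applies each upgrade, then refreshes the HUD.
; Health bonuses add flatly to max and current values, while damage, movement and projectile speed bonuses compound as percentage multipliers.
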(event `self.ReceiveBeginPlay`
  (bind _asbp_top_down_character (cast `/Game/CustomAguilar/Character/BP_TopDownCharacter` (`GameplayStatics.GetPlayerCharacter` 0)))
  (bind _output_get (set `self.PlayerRef` _asbp_top_down_character))
  (set `self.BaseWalkSpeed` (`CharacterMovementComponent.MaxWalkSpeed` (`Character.CharacterMovement` _output_get)))
  (bind _returnvalue (`|CreateWidget` "/Game/CustomAguilar/Widgets/WBP_UpgradeInventory.WBP_UpgradeInventory_C"))
  (bind _output_get_2 (set `self.InventoryHUDRef` _returnvalue))
  (`UserWidget.AddToViewport` _output_get_2 0))

(fn `AddUpgrade`
  (params (NewUpgrade :type "/Game/CustomAguilar/Upgrades/ST_UpgradeData Structure"))
  (bind _inventoryhudref (`self.InventoryHUDRef`))
  (if (< (`KismetArrayLibrary.Array_Length` (`self.UpgradeSlots`)) (`self.MaxSlots`))
    (`KismetArrayLibrary.Array_Add` (`self.UpgradeSlots`) NewUpgrade)
    (`self.ApplyUpgrade` NewUpgrade)
    (`/Engine/EditorBlueprintResources/StandardMacros.IsValid` _inventoryhudref
      (:`Is Valid`
        (`/Game/CustomAguilar/Widgets/WBP_UpgradeInventory.UpdateInventory` _inventoryhudref (`self.UpgradeSlots`))))))

(fn `ApplyUpgrade`
  (params (Upgrade :type "/Game/CustomAguilar/Upgrades/ST_UpgradeData Structure"))
  (bind (_upgradetype _upgradevalue) (break `/Game/CustomAguilar/Upgrades/ST_UpgradeData` Upgrade))
  (bind _bp_healthcomponent (`/Game/CustomAguilar/Character/BP_TopDownCharacter.BP_HealthComponent` (`self.PlayerRef`)))
  (switch `/Game/CustomAguilar/Upgrades/E_UpgradeType` _upgradetype
    (:`NewEnumerator0`
      (set `/Game/CustomAguilar/Components/BP_HealthComponent.MaxHealth` (+ (`/Game/CustomAguilar/Components/BP_HealthComponent.MaxHealth` _bp_healthcomponent) _upgradevalue) _bp_healthcomponent)
      (set `/Game/CustomAguilar/Components/BP_HealthComponent.CurrentHealth` (+ _upgradevalue (`/Game/CustomAguilar/Components/BP_HealthComponent.CurrentHealth` _bp_healthcomponent)) _bp_healthcomponent)
      (`KismetSystemLibrary.PrintString` "MAX HEALTH"))
    (:`NewEnumerator1`
      (bind _output_get (set `self.DamageMultiplier` (* (+ (/ _upgradevalue 100.0) 1.0) (`self.DamageMultiplier`))))
      (set `/Game/CustomAguilar/Character/BP_TopDownCharacter.DamageMultiplier` _output_get (`self.PlayerRef`))
      (`KismetSystemLibrary.PrintString` "DAMAGE"))
    (:`NewEnumerator2`
      (bind _output_get_2 (set `self.MovementSpeedMultplier` (* (+ (/ _upgradevalue 100.0) 1.0) (`self.MovementSpeedMultplier`))))
      (set `CharacterMovementComponent.MaxWalkSpeed` (* _output_get_2 (`self.BaseWalkSpeed`)) (`Character.CharacterMovement` (`self.PlayerRef`)))
      (`KismetSystemLibrary.PrintString` "SPEED"))
    (:`NewEnumerator3`
      (bind _output_get_3 (set `self.ProjectileSpeedMultiplier` (* (+ (/ _upgradevalue 100.0) 1.0) (`self.ProjectileSpeedMultiplier`))))
      (set `/Game/CustomAguilar/Character/BP_TopDownCharacter.ProjectileSpeedMultiplier` _output_get_3 (`self.PlayerRef`))
      (`KismetSystemLibrary.PrintString` "PROJECTILE SPEED"))))

(fn `UserConstructionScript`)