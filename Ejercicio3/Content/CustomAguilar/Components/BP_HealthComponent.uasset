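; BP_HealthComponent is a health component that tracks current health against a maximum and signals death.
; It starts at MaxHealth on BeginPlay, and ReceiveDamage subtracts damage, calling the OnDeath dispatcher whenever health is at or below zero.
; Damage is not clamped and has no already-dead guard, so further hits fire OnDeath again.
; Heal clamps between zero and MaxHealth, and both functions print the new value.
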(event `self.ReceiveBeginPlay`
  (set `self.CurrentHealth` (`self.MaxHealth`)))

(fn `Heal`
  (params (HealAmount :type "Float (double-precision)"))
  (bind _output_get (set `self.CurrentHealth` (`KismetMathLibrary.FClamp` (+ (`self.CurrentHealth`) HealAmount) 0.0 (`self.MaxHealth`))))
  (`KismetSystemLibrary.PrintString` (`KismetStringLibrary.Conv_DoubleToString` _output_get)))

(fn `ReceiveDamage`
  (params (DamageAmount :type "Float (double-precision)"))
  (bind _output_get (set `self.CurrentHealth` (- (`self.CurrentHealth`) DamageAmount)))
  (`KismetSystemLibrary.PrintString` (`KismetStringLibrary.Conv_DoubleToString` (`self.CurrentHealth`)))
  (if (<= _output_get 0.0)
    (`self.OnDeath`)))