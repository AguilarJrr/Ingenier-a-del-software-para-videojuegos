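; BP_NPCMerchant is a merchant NPC that opens the shop screen when interacted with.
; Interact creates a WBP_Shop widget, adds it to the viewport, shows the mouse cursor, switches the first player controller to UI-only input and pauses the game.
; The event graph holds only disabled default events, and nothing here closes the shop or unpauses the game.
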(fn `Interact`
  (bind _returnvalue (`GameplayStatics.GetPlayerController` 0))
  (bind _returnvalue_2 (`|CreateWidget` "/Game/CustomAguilar/Widgets/WBP_Shop.WBP_Shop_C"))
  (`UserWidget.AddToViewport` _returnvalue_2 0)
  (bind _output_get (set `PlayerController.bShowMouseCursor` true _returnvalue))
  (`WidgetBlueprintLibrary.SetInputMode_UIOnlyEx` _returnvalue null "DoNotLock" _output_get)
  (`GameplayStatics.SetGamePaused` true))

(fn `UserConstructionScript`
  (`parent.UserConstructionScript`))