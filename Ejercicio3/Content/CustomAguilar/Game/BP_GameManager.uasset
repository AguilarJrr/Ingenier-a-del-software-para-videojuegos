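; BP_GameManager runs a round-based enemy wave game, alternating combat rounds with rest phases until the final round completes.
; Each round loads limits from RoundConfigs, and a looping timer, set once at BeginPlay, asks BP_EnemySpawner for normal or strong enemies.
; Spawn and death events update counters and the round HUD, then check for round end.
; Rest spawns chests at BP_ChestSpawnPoint actors, and StartNextRound removes them and advances the round.
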(event `self.ReceiveBeginPlay`
  (set `self.GameState` "NewEnumerator0")
  (set `self.CurrentRound` 1)
  (bind _outactors (`GameplayStatics.GetAllActorsOfClass` "/Game/CustomAguilar/Enemies/BP_EnemySpawner.BP_EnemySpawner_C"))
  (set `self.EnemySpawnerRef` (`|GetArrayItem` _outactors))
  (`self.StartCurrentRound`)
  (bind _returnvalue (`|CreateWidget` "/Game/CustomAguilar/Widgets/WBP_RoundHUD.WBP_RoundHUD_C"))
  (bind _output_get (set `self.RoundHUDRef` _returnvalue))
  (`UserWidget.AddToViewport` _output_get 0)
  (bind _outactors_2 (`GameplayStatics.GetAllActorsOfClass` "/Game/CustomAguilar/Game/BP_ChestSpawnPoint.BP_ChestSpawnPoint_C"))
  (set `self.ChestSpawnPoints` _outactors_2)
  (`KismetSystemLibrary.K2_SetTimerDelegate` (delegate `HandleTrySpawnEnemy`) (`self.SpawnInterval`) true))

(event `HandleEnemyDied`
  (if (> (`self.AliveEnemies`) 0)
    (set `self.AliveEnemies` (- (`self.AliveEnemies`) 1))
    (`self.CheckRoundEnd`)
    (`/Game/CustomAguilar/Widgets/WBP_RoundHUD.UpdateHUD` (`self.RoundHUDRef`))))

(event `HandleTrySpawnEnemy`
  (`self.TrySpawnEnemy`))

(event `TrySpawnEnemy`
  (if (and (< (`self.EnemiesSpawned`) (`self.EnemiesToSpawn`)) (< (`self.AliveEnemies`) (`self.MaxAliveEnemies`)))
    (`/Game/CustomAguilar/Enemies/BP_EnemySpawner.SpawnEnemy` (`self.EnemySpawnerRef`) (< (`KismetMathLibrary.RandomFloatInRange` 0.0 100.0) (`self.StrongEnemyChance`)))))

(event `HandleEnemySpawned`
  (set `self.EnemiesSpawned` (+ (`self.EnemiesSpawned`) 1))
  (set `self.AliveEnemies` (+ (`self.AliveEnemies`) 1))
  (`self.CheckRoundEnd`)
  (`/Game/CustomAguilar/Widgets/WBP_RoundHUD.UpdateHUD` (`self.RoundHUDRef`)))

(event `CheckRoundEnd`
  (if (and (>= (`self.EnemiesSpawned`) (`self.EnemiesToSpawn`)) (== (`self.AliveEnemies`) 0))
    (`self.StartRest`)))

(event `StartRest`
  (if (< (`self.CurrentRound`) (`self.TotalRounds`))
    (set `self.GameState` "NewEnumerator1")
    (`KismetSystemLibrary.PrintString` "RONDA COMPLETADA")
    (`self.SpawnChests`)
    (else
      (set `self.GameState` "NewEnumerator2")
      (`KismetSystemLibrary.PrintString` "HAS COMPLETADO TODAS LAS RONDAS"))))

(event `StartNextRound`
  (if (and (== (`self.GameState`) 1) (< (`self.CurrentRound`) (`self.TotalRounds`)))
    (set `self.CurrentRound` (+ (`self.CurrentRound`) 1))
    (`self.RemoveSpawnedChests`)
    (`self.StartCurrentRound`)
    (set `self.GameState` "NewEnumerator0")
    (`KismetSystemLibrary.PrintString` "EMPEZANDO RONDA")
    (`/Game/CustomAguilar/Widgets/WBP_RoundHUD.UpdateHUD` (`self.RoundHUDRef`))
    (else
      (`KismetSystemLibrary.PrintString` "NO HA ACABADO LA RONDA TODAVÍA"))))

(event `SpawnChests`
  (for _array_element (`self.ChestSpawnPoints`)
    (bind _returnvalue (`|SpawnActorFromClass` (`self.ChestClass`) (`self.GetTransform` _array_element) "Undefined" "MultiplyWithRoot" null null))
    (`KismetArrayLibrary.Array_Add` (`self.SpawnedChest`) _returnvalue)))

(event `RemoveSpawnedChests`
  (for _array_element (`self.SpawnedChest`)
    (`self.K2_DestroyActor` _array_element))
  (`KismetArrayLibrary.Array_Clear` (`self.SpawnedChest`)))

(fn `StartCurrentRound`
  (bind _roundhudref (`self.RoundHUDRef`))
  (bind (_enemiesperround _maxaliveenemies _spawninterval _strongenemychance) (break `/Game/CustomAguilar/Game/ST_RoundConfig` (`|GetArrayItem` (`self.RoundConfigs`) (- (`self.CurrentRound`) 1))))
  (set `self.EnemiesToSpawn` _enemiesperround)
  (set `self.EnemiesSpawned` 0)
  (set `self.AliveEnemies` 0)
  (set `self.MaxAliveEnemies` _maxaliveenemies)
  (set `self.SpawnInterval` _spawninterval)
  (`/Game/CustomAguilar/Enemies/BP_EnemySpawner.SetRoundSettings` (`self.EnemySpawnerRef`) _strongenemychance)
  (`/Engine/EditorBlueprintResources/StandardMacros.IsValid` _roundhudref
    (:`Is Valid`
      (`/Game/CustomAguilar/Widgets/WBP_RoundHUD.UpdateHUD` _roundhudref))))

(fn `UserConstructionScript`)