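; BP_Button is an interactable button that starts the next round.
; Interact calls its parent, then takes the first BP_GameManager found in the level and calls StartNextRound on it.
; Actor overlap prints a "¿NUEVA RONDA?" (new round?) prompt via PrintString.
; Leftover nodes for opening a TargetDoor and destroying the actor are disconnected and never run.
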(event `self.ReceiveActorBeginOverlap`
  (params (OtherActor :type "Actor Object Reference"))
  (`parent.ReceiveActorBeginOverlap` OtherActor)
  (`KismetSystemLibrary.PrintString` "¿NUEVA RONDA?"))

(fn `Interact`
  (`parent.Interact`)
  (bind _outactors (`GameplayStatics.GetAllActorsOfClass` "/Game/CustomAguilar/Game/BP_GameManager.BP_GameManager_C"))
  (`/Game/CustomAguilar/Game/BP_GameManager.StartNextRound` (`|GetArrayItem` _outactors)))

(fn `UserConstructionScript`
  (`parent.UserConstructionScript`))