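; BP_Chest is an interactable chest that offers the player a random upgrade the first time it is opened.
; Interact calls OpenChest, which snaps the lid open, sets IsOpen to block repeats, and picks a random DT_Upgrades row.
; It then shows WBP_UpgradeChoice, passing in that upgrade and the first BP_UpgradeInventory found in the level.
; The chest's own AddUpgrade call is unwired.
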(fn `Interact`
  (`self.OpenChest`))

(fn `OpenChest`
  (if (not (`self.IsOpen`))
    (`SceneComponent.K2_SetRelativeRotation` (`self.ChestLid`) (struct :`Roll` -70.0) false false)
    (set `self.IsOpen` true)
    (bind _outrownames (`DataTableFunctionLibrary.GetDataTableRowNames` "/Game/CustomAguilar/Upgrades/DT_Upgrades.DT_Upgrades"))
    (bind _returnvalue (`|GetDataTableRow` "/Game/CustomAguilar/Upgrades/DT_Upgrades.DT_Upgrades" (`|GetArrayItem` _outrownames (`KismetMathLibrary.RandomIntegerInRange` 0 (- (`KismetArrayLibrary.Array_Length` _outrownames) 1))))
      (:`then`
        (bind _outactors (`GameplayStatics.GetAllActorsOfClass` "/Game/CustomAguilar/Upgrades/BP_UpgradeInventory.BP_UpgradeInventory_C"))
        (bind _returnvalue_2 (`|CreateWidget` "/Game/CustomAguilar/Widgets/WBP_UpgradeChoice.WBP_UpgradeChoice_C" (`GameplayStatics.GetPlayerController` 0) _returnvalue (`|GetArrayItem` _outactors)))
        (`UserWidget.AddToViewport` _returnvalue_2 0)))))

(fn `UserConstructionScript`
  (`parent.UserConstructionScript`))