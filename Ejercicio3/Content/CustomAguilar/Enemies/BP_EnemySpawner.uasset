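; BP_EnemySpawner is an actor that spawns weak or strong enemies at unlocked spawn points.
; On BeginPlay it caches all BP_EnemySpawnPoint actors and the first BP_GameManager.
; SpawnEnemy picks a random unlocked point, selects the class from a boolean, binds the enemy's death event and notifies the manager of the spawn.
; SetRoundSettings writes the strong enemy chance to the game manager.
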(event `self.ReceiveBeginPlay`
  (bind _outactors (`GameplayStatics.GetAllActorsOfClass` "/Game/CustomAguilar/Enemies/BP_EnemySpawnPoint.BP_EnemySpawnPoint_C"))
  (set `self.SpawnPoints` _outactors)
  (bind _outactors_2 (`GameplayStatics.GetAllActorsOfClass` "/Game/CustomAguilar/Game/BP_GameManager.BP_GameManager_C"))
  (set `self.GameManagerRef` (`|GetArrayItem` _outactors_2)))

(fn `SetRoundSettings`
  (params (NewStrongEnemyChance :type "Float (double-precision)"))
  (set `/Game/CustomAguilar/Game/BP_GameManager.StrongEnemyChance` NewStrongEnemyChance (`self.GameManagerRef`)))

(fn `SpawnEnemy`
  (params (SpawnStrongEnemy :type Boolean :default false))
  (bind _returnvalue (`KismetArrayLibrary.Array_Length` (`self.AvailableSpawnPoints`)))
  (`KismetArrayLibrary.Array_Clear` (`self.AvailableSpawnPoints`))
  (for _array_element (`self.SpawnPoints`)
    (if (`/Game/CustomAguilar/Enemies/BP_EnemySpawnPoint.IsUnlocked` _array_element)
      (`KismetArrayLibrary.Array_Add` (`self.AvailableSpawnPoints`) _array_element)))
  (if (> _returnvalue 0)
    (if (`local.SpawnStrongEnemy`)
      (set `self.SelectedEnemyClass` (`self.StrongEnemyClass`))
      (else
        (set `self.SelectedEnemyClass` (`self.WeakEnemyClass`))))
    (bind _returnvalue_2 (`|SpawnActorFromClass` (`self.SelectedEnemyClass`) (`self.GetTransform` (`|GetArrayItem` (`self.AvailableSpawnPoints`) (`KismetMathLibrary.RandomIntegerInRange` 0 (- _returnvalue 1)))) "Undefined" "MultiplyWithRoot" null null))
    (`/Engine/EditorBlueprintResources/StandardMacros.IsValid` _returnvalue_2
      (:`Is Valid`
        (add `/Game/CustomAguilar/Enemies/BP_EnemyBase.OnEnemyDied` _returnvalue_2 (`|CreateDelegate` (`self.GameManagerRef`) :!event `HandleEnemyDied`))
        (`/Game/CustomAguilar/Game/BP_GameManager.HandleEnemySpawned` (`self.GameManagerRef`))))))

(fn `UserConstructionScript`)