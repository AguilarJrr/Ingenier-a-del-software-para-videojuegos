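; Base enemy for a top-down game that chases the player, deals contact damage and can drop health on death.
; Perseguir runs AI MoveTo toward the player and restarts one second after each success or failure.
; Capsule hits on the player character apply damage through the damage component, gated by a timer-reset cooldown.
; The health component's death event fires OnEnemyDied, destroys the actor and randomly spawns a health pickup.
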(event `Perseguir`
  (`|AIMoveTo` self (0.0 0.0 0.0) (`GameplayStatics.GetPlayerCharacter` 0)
    (:`OnSuccess`
      _)
    (:`OnFail`
      _))
  (`KismetSystemLibrary.Delay` 1.0)
  (`self.Perseguir`))

(event `self.CapsuleComponent.OnComponentHit`
  (params (HitComponent :type "PrimitiveComponent Object Reference") (OtherActor :type "Actor Object Reference") (OtherComp :type "PrimitiveComponent Object Reference") (NormalImpulse :type "Vector Structure") (Hit :type "HitResult Structure (by ref)"))
  (bind _asbp_top_down_character (cast `/Game/CustomAguilar/Character/BP_TopDownCharacter` OtherActor))
  (if (`self.CanDamagePlayer`)
    (set `self.CanDamagePlayer` false)
    (`/Game/CustomAguilar/Components/BP_DamageComponent.GetDamage` (`self.BP_DamageComponent`) _asbp_top_down_character)
    (`KismetSystemLibrary.K2_SetTimerDelegate` (delegate `ResetDamageCoolDown`) (`self.DamageCoolDown`))))

(event `ResetDamageCoolDown`
  (set `self.CanDamagePlayer` true))

(event `EnemyDeath`
  (`self.OnEnemyDied`)
  (`self.K2_DestroyActor`)
  (if (<= (`KismetMathLibrary.RandomFloatInRange` 0.0 100.0) (`self.HealthPickupDropChance`))
    (`|SpawnActorFromClass` "/Game/CustomAguilar/Game/BP_HealthPickup.BP_HealthPickup_C" (`self.GetTransform`) "Undefined" "MultiplyWithRoot" null null)))

(event `self.ReceiveBeginPlay`
  (add `/Game/CustomAguilar/Components/BP_HealthComponent.OnDeath` (`self.BP_HealthComponent`) (delegate `HandleEnemyDeath`))
  (`self.Perseguir`))

(event `HandleEnemyDeath`
  (`self.EnemyDeath`))

(fn `UserConstructionScript`)