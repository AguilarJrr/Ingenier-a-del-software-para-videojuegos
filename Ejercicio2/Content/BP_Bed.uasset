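; BP_Bed is an interactable bed that heals the player.
; Its Interact function casts player character 0 to BP_TopDownCharacter, calls Heal with HealAmount, and prints a Spanish confirmation message ("Te has curado").
; The event graph holds only disabled default events, and the construction script just calls its parent.
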(fn `Interact`
  (bind _asbp_top_down_character (cast `/Game/TopDown/Blueprints/BP_TopDownCharacter` (`GameplayStatics.GetPlayerCharacter` 0)))
  (`/Game/TopDown/Blueprints/BP_TopDownCharacter.Heal` _asbp_top_down_character (`self.HealAmount`))
  (`KismetSystemLibrary.PrintString` "Te has curado"))

(fn `UserConstructionScript`
  (`parent.UserConstructionScript`))